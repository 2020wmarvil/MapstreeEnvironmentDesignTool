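; Inventory actor for the Mapstree editor that holds a fixed number of item-class slots and displays them on screen.
; On BeginPlay it enables input, sizes the slot array and creates the W_MapstreeEditor widget with a reference to itself.
; AddItem fills the first empty slot and refreshes only that slot's widget, with key 1 as a debug trigger.
; Item info is read from class defaults, so slots store no item instances.
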(event `Key|One`
  (params (Key :type "Key Structure"))
  (:`Pressed`
    (bind _success (`self.AddItem` (`self.Item Class`)))
    (`KismetSystemLibrary.PrintString` (`KismetStringLibrary.Conv_BoolToString` _success))))

(event `self.ReceiveBeginPlay`
  (`self.EnableInput` (`GameplayStatics.GetPlayerController` 0))
  (`KismetArrayLibrary.Array_Resize` (`self.Slots`) (`self.AmountOfSlots`))
  (bind _returnvalue (`|CreateWidget` "/Game/Blueprints/MapstreeEditor/W_MapstreeEditor.W_MapstreeEditor_C" null self (`self.Slots Per Row`)))
  (bind _output_get (set `self.EditorWidget` _returnvalue))
  (set `self.InventoryWidget` (`/Game/Blueprints/MapstreeEditor/W_MapstreeEditor.InventoryWidget` _output_get))
  (`UserWidget.AddToViewport` (`self.EditorWidget`) 0))

(event `UpdateSlotAtIndex`
  (params (Index :type Integer))
  (`/Game/Blueprints/MapstreeEditor/W_InventorySLot.UpdateSlot` (`|GetArrayItem` (`/Game/Blueprints/MapstreeEditor/W_Inventory.SlotsWidgets` (`self.InventoryWidget`)) Index)))

(fn `AddItem`
  (params (ItemClass :type "/Game/Blueprints/MapstreeEditor/BP_MasterItem Object Reference"))
  (returns (Success :type Boolean))
  (locals (localClass :type "/Game/Blueprints/MapstreeEditor/BP_MasterItem Object Reference") (FoundIndex :type Integer))
  (set `local.localClass` ItemClass)
  (bind (_success _index) (`self.SearchEmptySlot`))
  (if _success
    (bind _output_get (set `local.FoundIndex` _index))
    (`KismetArrayLibrary.Array_Set` (`self.Slots`) _output_get (make `/Game/Blueprints/MapstreeEditor/S_InventorySlot` (`GameplayStatics.GetObjectClass` (`local.localClass`))))
    (`self.UpdateSlotAtIndex` (`local.FoundIndex`))
    (return true)
    (else
      (return false))))

(fn `GetItemInfoAtIndex`
  (params (Index :type Integer))
  (returns (Empty :type Boolean) (ItemInfo :type "/Game/Blueprints/MapstreeEditor/ItemInfo Structure"))
  (bind _itemclass (break `/Game/Blueprints/MapstreeEditor/S_InventorySlot` (`|GetArrayItem` (`self.Slots`) Index)))
  (if (`KismetSystemLibrary.IsValidClass` _itemclass)
    (return false (defaults `Object` _itemclass))
    (else
      (return true))))

(fn `IsSlotEmpty`
  (params (Index :type Integer))
  (returns (Empty :type Boolean))
  (return (not (`KismetSystemLibrary.IsValidClass` (`.ItemClass_2_43C8644040961CF9686609A737E6252A` (break `/Game/Blueprints/MapstreeEditor/S_InventorySlot` (`|GetArrayItem` (`self.Slots`) Index)))))))

(fn `SearchEmptySlot`
  (returns (Success :type Boolean) (Index :type Integer))
  (locals (localBool :type Boolean) (localIndex :type Integer))
  (for (_array_element _array_index) (`self.Slots`)
    (if (not (`KismetSystemLibrary.IsValidClass` (`.ItemClass_2_43C8644040961CF9686609A737E6252A` (break `/Game/Blueprints/MapstreeEditor/S_InventorySlot` _array_element))))
      (set `local.localBool` true)
      (set `local.localIndex` _array_index)
      (break)))
  (return (`local.localBool`) (`local.localIndex`)))

(fn `UserConstructionScript`)